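; BP_Closet is a closet actor that swings open on a button trigger and closes on overlap, intended for the player's hand.
; The OpenCloset event plays a timeline that lerps the Closet component's relative rotation through a quarter turn.
; Any actor overlap while open reverses the same timeline, since the overlapping actor is not filtered.
; An IsOpen flag guards both triggers against repeats.
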(event Custom|OpenCloset
  ;[0.15 0.15 0.15 0.5] Opening closet with button (trigger and logic)
  (if (not (Variables|Default|GetIsOpen))
    (Variables|Default|SetIsOpen true)
    ;[0.15 0.15 0.15 0.5] Closet animation (opening and closing)
    (bind _rotation (Timeline|Timeline%20Animation Play)
      (:Update
        (Transformation|SetRelativeRotation (Variables|Default|GetCloset) (Math|Rotator|Lerp(Rotator) "0, 0, 0" "0.000000,-90.000000,0.000000" _rotation) false false)))))

(event Collision|EventActorBeginOverlap
  (params (OtherActor :type Actor%20Object%20Reference))
  ;[0.15 0.15 0.15 0.5] Closing closet with hand (trigger and logic)
  (if (Variables|Default|GetIsOpen)
    (Variables|Default|SetIsOpen false)
    ;[0.15 0.15 0.15 0.5] Closet animation (opening and closing)
    (bind _rotation (Timeline|Timeline%20Animation Reverse)
      (:Update
        (Transformation|SetRelativeRotation (Variables|Default|GetCloset) (Math|Rotator|Lerp(Rotator) "0, 0, 0" "0.000000,-90.000000,0.000000" _rotation) false false)))))

(fn ConstructionScript)