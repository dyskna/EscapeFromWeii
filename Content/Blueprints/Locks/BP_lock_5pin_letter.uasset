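; Five-button letter combination lock for a puzzle, worked by collision overlaps.
; The first overlap on the lock reveals the hidden buttons, and later overlaps compare the five button values to the correct order.
; Each button overlap cycles through ten letters, replacing the spawned letter actor via NumberSpwan.
; A match destroys the letters and lock, then opens the linked closet drawer or numbered drawer and its hinge, chosen by which reference is valid.
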(event OnComponentBeginOverlap(Lock_Colision)
  (params (OverlappedComponent :type Primitive%20Component%20Object%20Reference) (OtherActor :type Actor%20Object%20Reference) (OtherComp :type Primitive%20Component%20Object%20Reference) (OtherBodyIndex :type Integer) (bFromSweep :type Boolean) (SweepResult :type Hit%20Result%20Structure%20%28by%20ref%29))
  (bind _button1_value (Variables|Default|GetButton1_value))
  (bind _button2_value (Variables|Default|GetButton2_value))
  (bind _button3_value (Variables|Default|GetButton3_value))
  (bind _button4_value (Variables|Default|GetButton4_value))
  (bind _button5_value (Variables|Default|GetButton5_value))
  (bind _bp_drawer_num (Variables|References|GetBP_Drawer_Num))
  (bind _bp_small_closet_downref (Variables|References|GetBP_small_closet_downRef))
  (bind _array (Utilities|Array|MakeArray _button1_value _button2_value _button3_value _button4_value _button5_value))
  (if (Variables|Default|GetHide)
    (Rendering|SetVisibility (Utilities|Array|MakeArray (Variables|Default|GetButton1) (Variables|Default|GetButton2) (Variables|Default|GetButton3) (Variables|Default|GetButton4) (Variables|Default|GetButton5)) true false)
    (Collision|SetCollisionEnabled (Utilities|Array|MakeArray (Variables|Default|GetButton1_Colision) (Variables|Default|GetButton2_Colision) (Variables|Default|GetButton3_Colision) (Variables|Default|GetButton4_Colision) (Variables|Default|GetButton5_Colision)) "QueryAndPhysics")
    (Variables|Default|SetHide false)
    (else
      ;[0.15 0.15 0.15 0.5] compare
      (if (Utilities|Array|Identical (Variables|Default|GetButtons_Order_correct) _array)
        ;[0.15 0.15 0.15 0.5] hologram remove
        (Actor|DestroyActor (Variables|Default|GetButton4_number))
        (Actor|DestroyActor)
        ;[0.15 0.15 0.15 0.5] After correctly solving the lock
        (if (Utilities|IsValid _bp_small_closet_downref) ; When adding more locks of this type, branch off of False
          (Default|OpenDrawerDown _bp_small_closet_downref "0.000000,50.000000,0.000000")
          (Default|MoveButton (Variables|References|GetButton_Start_ColorsRef) "0.000000,-50.000000,0.000000")
          (Default|OpenHinge (Variables|References|GetHingeRef))
          (else
            ;[0.15 0.15 0.15 0.5] After correctly solving the lock
            (if (Utilities|IsValid _bp_drawer_num) ; When adding more locks of this type, branch off of False
              (Default|OpenDrawer _bp_drawer_num "0.000000,50.000000,0.000000")
              (Default|OpenHinge (Variables|References|GetHingeRef)))))
        (else
          (Utilities|Array|Clear _array))))))

(event OnComponentBeginOverlap(Button1_Colision)
  (params (OverlappedComponent :type Primitive%20Component%20Object%20Reference) (OtherActor :type Actor%20Object%20Reference) (OtherComp :type Primitive%20Component%20Object%20Reference) (OtherBodyIndex :type Integer) (bFromSweep :type Boolean) (SweepResult :type Hit%20Result%20Structure%20%28by%20ref%29))
  ;[0.15 0.15 0.15 0.5] Number Spawn
  (bind (_buttonnumber _buttonvalue) (CallFunction|NumberSpwan (Variables|Default|GetButton1_number) (Variables|Default|GetButton1) (Variables|Default|GetButton1_value)))
  (Variables|Default|SetButton1_number _buttonnumber)
  (Variables|Default|SetButton1_value _buttonvalue))

(event OnComponentBeginOverlap(Button2_Colision)
  (params (OverlappedComponent :type Primitive%20Component%20Object%20Reference) (OtherActor :type Actor%20Object%20Reference) (OtherComp :type Primitive%20Component%20Object%20Reference) (OtherBodyIndex :type Integer) (bFromSweep :type Boolean) (SweepResult :type Hit%20Result%20Structure%20%28by%20ref%29))
  ;[0.15 0.15 0.15 0.5] Number Spawn
  (bind (_buttonnumber _buttonvalue) (CallFunction|NumberSpwan (Variables|Default|GetButton2_number) (Variables|Default|GetButton2) (Variables|Default|GetButton2_value)))
  (Variables|Default|SetButton2_number _buttonnumber)
  (Variables|Default|SetButton2_value _buttonvalue))

(event OnComponentBeginOverlap(Button3_Colision)
  (params (OverlappedComponent :type Primitive%20Component%20Object%20Reference) (OtherActor :type Actor%20Object%20Reference) (OtherComp :type Primitive%20Component%20Object%20Reference) (OtherBodyIndex :type Integer) (bFromSweep :type Boolean) (SweepResult :type Hit%20Result%20Structure%20%28by%20ref%29))
  ;[0.15 0.15 0.15 0.5] Number Spawn
  (bind (_buttonnumber _buttonvalue) (CallFunction|NumberSpwan (Variables|Default|GetButton3_number) (Variables|Default|GetButton3) (Variables|Default|GetButton3_value)))
  (Variables|Default|SetButton3_number _buttonnumber)
  (Variables|Default|SetButton3_value _buttonvalue))

(event OnComponentBeginOverlap(Button4_Colision)
  (params (OverlappedComponent :type Primitive%20Component%20Object%20Reference) (OtherActor :type Actor%20Object%20Reference) (OtherComp :type Primitive%20Component%20Object%20Reference) (OtherBodyIndex :type Integer) (bFromSweep :type Boolean) (SweepResult :type Hit%20Result%20Structure%20%28by%20ref%29))
  ;[0.15 0.15 0.15 0.5] Number Spawn
  (bind (_buttonnumber _buttonvalue) (CallFunction|NumberSpwan (Variables|Default|GetButton4_number) (Variables|Default|GetButton4) (Variables|Default|GetButton4_value)))
  (Variables|Default|SetButton4_number _buttonnumber)
  (Variables|Default|SetButton4_value _buttonvalue))

(event OnComponentBeginOverlap(Button5_Colision)
  (params (OverlappedComponent :type Primitive%20Component%20Object%20Reference) (OtherActor :type Actor%20Object%20Reference) (OtherComp :type Primitive%20Component%20Object%20Reference) (OtherBodyIndex :type Integer) (bFromSweep :type Boolean) (SweepResult :type Hit%20Result%20Structure%20%28by%20ref%29))
  ;[0.15 0.15 0.15 0.5] Number Spawn
  (bind (_buttonnumber _buttonvalue) (CallFunction|NumberSpwan (Variables|Default|GetButton5_number) (Variables|Default|GetButton5) (Variables|Default|GetButton5_value)))
  (Variables|Default|SetButton5_number _buttonnumber)
  (Variables|Default|SetButton5_value _buttonvalue))

(event EventBeginPlay
  (Rendering|SetVisibility (Utilities|Array|MakeArray (Variables|Default|GetButton1) (Variables|Default|GetButton2) (Variables|Default|GetButton3) (Variables|Default|GetButton4) (Variables|Default|GetButton5)) false false)
  (Collision|SetCollisionEnabled (Utilities|Array|MakeArray (Variables|Default|GetButton1_Colision) (Variables|Default|GetButton2_Colision) (Variables|Default|GetButton3_Colision) (Variables|Default|GetButton4_Colision) (Variables|Default|GetButton5_Colision)) "NoCollision"))

(fn ConstructionScript)

(fn NumberSpwan
  (params (Button_number :type Actor%20Object%20Reference) (Button :type Primitive%20Component%20Object%20Reference) (Button_value :type Integer))
  (bind _returnvalue (Transformation|GetWorldRotation Button))
  (bind _output_get (Variables|Default|SetNumber_Spawn_value Button_value))
  (if (Utilities|IsValid Button_number)
    (Actor|DestroyActor Button_number))
  (bind _returnvalue_2 (Game|SpawnActorfromClass (Utilities|Array|Get(acopy) (Variables|Default|GetLetter) _output_get) (Math|Transform|MakeTransform (Transformation|GetWorldLocation Button) (Math|Rotator|MakeRotator (- (.roll _returnvalue) 9e+01) (.pitch _returnvalue) (.yaw _returnvalue)) "1.000000,1.000000,1.000000") "Undefined" "MultiplyWithRoot" 0 0))
  (if (== 9 _output_get)
    (Variables|Default|SetNumber_Spawn_value 0)
    (else
      (bind _output_get_2 (Variables|Default|SetNumber_Spawn_value (+ 1 _output_get)))))
  (return _returnvalue_2 _output_get_2))