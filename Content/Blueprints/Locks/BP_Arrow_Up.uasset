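; Up arrow for a lock that cycles the digit in its slot forward through 0 to 9.
; Any overlap with its Box destroys the current Slot actor and spawns the Num_0 to Num_9 class matching Value just below the Arrow.
; An if/else chain picks the class, then Value increments after the spawn, wrapping to 0 after 9, so it holds the next digit rather than the displayed one.
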(event OnComponentBeginOverlap(Box)
  (params (OverlappedComponent :type Primitive%20Component%20Object%20Reference) (OtherActor :type Actor%20Object%20Reference) (OtherComp :type Primitive%20Component%20Object%20Reference) (OtherBodyIndex :type Integer) (bFromSweep :type Boolean) (SweepResult :type Hit%20Result%20Structure%20%28by%20ref%29))
  (if (== (Variables|Default|Getvalue) 0)
    (Actor|DestroyActor (Variables|Default|Getslot))
    (bind _returnvalue (Game|SpawnActorfromClass "/Game/Blueprints/Locks/Numbers/Num_0.Num_0_C" (Math|Transform|MakeTransform (- (Transformation|GetWorldLocation (Variables|Default|GetArrow)) "0.000000,0.000000,36.000000") "0, 0, 0" "1.000000,1.000000,1.000000") "Undefined" "MultiplyWithRoot" 0 0))
    (Variables|Default|Setslot _returnvalue)
    (Variables|Default|Setvalue (+ (Variables|Default|Getvalue) 1) :!label _label)
    (elif (== (Variables|Default|Getvalue) 1)
      (Actor|DestroyActor (Variables|Default|Getslot))
      (bind _returnvalue_2 (Game|SpawnActorfromClass "/Game/Blueprints/Locks/Numbers/Num_1.Num_1_C" (Math|Transform|MakeTransform (- (Transformation|GetWorldLocation (Variables|Default|GetArrow)) "0.000000,0.000000,36.000000") "0, 0, 0" "1.000000,1.000000,1.000000") "Undefined" "MultiplyWithRoot" 0 0))
      (Variables|Default|Setslot _returnvalue_2)
      (goto _label)
      (elif (== (Variables|Default|Getvalue) 2)
        (Actor|DestroyActor (Variables|Default|Getslot))
        (bind _returnvalue_3 (Game|SpawnActorfromClass "/Game/Blueprints/Locks/Numbers/Num_2.Num_2_C" (Math|Transform|MakeTransform (- (Transformation|GetWorldLocation (Variables|Default|GetArrow)) "0.000000,0.000000,36.000000") "0, 0, 0" "1.000000,1.000000,1.000000") "Undefined" "MultiplyWithRoot" 0 0))
        (Variables|Default|Setslot _returnvalue_3)
        (goto _label)
        (elif (== (Variables|Default|Getvalue) 3)
          (Actor|DestroyActor (Variables|Default|Getslot))
          (bind _returnvalue_4 (Game|SpawnActorfromClass "/Game/Blueprints/Locks/Numbers/Num_3.Num_3_C" (Math|Transform|MakeTransform (- (Transformation|GetWorldLocation (Variables|Default|GetArrow)) "0.000000,0.000000,36.000000") "0, 0, 0" "1.000000,1.000000,1.000000") "Undefined" "MultiplyWithRoot" 0 0))
          (Variables|Default|Setslot _returnvalue_4)
          (goto _label)
          (elif (== (Variables|Default|Getvalue) 4)
            (Actor|DestroyActor (Variables|Default|Getslot))
            (bind _returnvalue_5 (Game|SpawnActorfromClass "/Game/Blueprints/Locks/Numbers/Num_4.Num_4_C" (Math|Transform|MakeTransform (- (Transformation|GetWorldLocation (Variables|Default|GetArrow)) "0.000000,0.000000,36.000000") "0, 0, 0" "1.000000,1.000000,1.000000") "Undefined" "MultiplyWithRoot" 0 0))
            (Variables|Default|Setslot _returnvalue_5)
            (goto _label)
            (elif (== (Variables|Default|Getvalue) 5)
              (Actor|DestroyActor (Variables|Default|Getslot))
              (bind _returnvalue_6 (Game|SpawnActorfromClass "/Game/Blueprints/Locks/Numbers/Num_5.Num_5_C" (Math|Transform|MakeTransform (- (Transformation|GetWorldLocation (Variables|Default|GetArrow)) "0.000000,0.000000,36.000000") "0, 0, 0" "1.000000,1.000000,1.000000") "Undefined" "MultiplyWithRoot" 0 0))
              (Variables|Default|Setslot _returnvalue_6)
              (goto _label)
              (elif (== (Variables|Default|Getvalue) 6)
                (Actor|DestroyActor (Variables|Default|Getslot))
                (bind _returnvalue_7 (Game|SpawnActorfromClass "/Game/Blueprints/Locks/Numbers/Num_6.Num_6_C" (Math|Transform|MakeTransform (- (Transformation|GetWorldLocation (Variables|Default|GetArrow)) "0.000000,0.000000,36.000000") "0, 0, 0" "1.000000,1.000000,1.000000") "Undefined" "MultiplyWithRoot" 0 0))
                (Variables|Default|Setslot _returnvalue_7)
                (goto _label)
                (elif (== (Variables|Default|Getvalue) 7)
                  (Actor|DestroyActor (Variables|Default|Getslot))
                  (bind _returnvalue_8 (Game|SpawnActorfromClass "/Game/Blueprints/Locks/Numbers/Num_7.Num_7_C" (Math|Transform|MakeTransform (- (Transformation|GetWorldLocation (Variables|Default|GetArrow)) "0.000000,0.000000,36.000000") "0, 0, 0" "1.000000,1.000000,1.000000") "Undefined" "MultiplyWithRoot" 0 0))
                  (Variables|Default|Setslot _returnvalue_8)
                  (goto _label)
                  (elif (== (Variables|Default|Getvalue) 8)
                    (Actor|DestroyActor (Variables|Default|Getslot))
                    (bind _returnvalue_9 (Game|SpawnActorfromClass "/Game/Blueprints/Locks/Numbers/Num_8.Num_8_C" (Math|Transform|MakeTransform (- (Transformation|GetWorldLocation (Variables|Default|GetArrow)) "0.000000,0.000000,36.000000") "0, 0, 0" "1.000000,1.000000,1.000000") "Undefined" "MultiplyWithRoot" 0 0))
                    (Variables|Default|Setslot _returnvalue_9)
                    (goto _label)
                    (elif (== (Variables|Default|Getvalue) 9)
                      (Actor|DestroyActor (Variables|Default|Getslot))
                      (bind _returnvalue_10 (Game|SpawnActorfromClass "/Game/Blueprints/Locks/Numbers/Num_9.Num_9_C" (Math|Transform|MakeTransform (- (Transformation|GetWorldLocation (Variables|Default|GetArrow)) "0.000000,0.000000,36.000000") "0, 0, 0" "1.000000,1.000000,1.000000") "Undefined" "MultiplyWithRoot" 0 0))
                      (Variables|Default|Setslot _returnvalue_10)
                      (Variables|Default|Setvalue 0))))))))))))

(fn ConstructionScript)