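; Padlock number button that cycles a displayed digit from 0 to 9 each time something overlaps its Box trigger.
; Each overlap destroys the current Slot actor, spawns the class at index Value of the Numbers array at the Button's location, then increments Value, wrapping after 9.
; DestroyNumbers removes the shown digit and the button itself.
; An older per-digit branch chain remains in the graph, unconnected.
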(event OnComponentBeginOverlap(Box)
  (params (OverlappedComponent :type Primitive%20Component%20Object%20Reference) (OtherActor :type Actor%20Object%20Reference) (OtherComp :type Primitive%20Component%20Object%20Reference) (OtherBodyIndex :type Integer) (bFromSweep :type Boolean) (SweepResult :type Hit%20Result%20Structure%20%28by%20ref%29))
  ;[0.15 0.15 0.15 0.5] Number Spawn
  (if (Utilities|IsValid (Variables|Default|GetSlot))
    (Actor|DestroyActor (Variables|Default|Getslot)))
  (bind _returnvalue (Game|SpawnActorfromClass (Utilities|Array|Get(acopy) (Variables|Default|GetNumbers) (Variables|Default|Getvalue)) (Math|Transform|MakeTransform (Transformation|GetWorldLocation (Variables|Default|GetButton)) "0, 0, 0" "1.000000,1.000000,1.000000") "Undefined" "MultiplyWithRoot" 0 0))
  (Variables|Default|Setslot _returnvalue)
  (if (== 9 (Variables|Default|Getvalue))
    (Variables|Default|SetValue 0)
    (else
      (Variables|Default|Setvalue (+ (Variables|Default|Getvalue) 1)))))

(fn ConstructionScript)

(fn DestroyNumbers
  (Actor|DestroyActor (Variables|Default|GetSlot))
  (Actor|DestroyActor))