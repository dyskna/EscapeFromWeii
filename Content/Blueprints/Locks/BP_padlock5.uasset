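; BP_padlock5 is a number combination padlock, driven by overlaps on its Box.
; The first overlap teleports the Slots number buttons to offsets from the padlock.
; Later overlaps collect their values into Pattern and, after a short Delay, compare it with CorrectPattern.
; A match calls DestroyNumbers on the first five number buttons found in the level and ends the puzzle; a mismatch clears Pattern.
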(event OnComponentBeginOverlap(Box)
  (params (OverlappedComponent :type Primitive%20Component%20Object%20Reference) (OtherActor :type Actor%20Object%20Reference) (OtherComp :type Primitive%20Component%20Object%20Reference) (OtherBodyIndex :type Integer) (bFromSweep :type Boolean) (SweepResult :type Hit%20Result%20Structure%20%28by%20ref%29))
  (bind _padlock (Variables|Default|Getpadlock))
  (bind _pattern (Variables|Default|GetPattern))
  (if (not (Variables|Default|GetEnd))
    (if (Variables|Default|GetIs_Spawned)
      ;[0.15 0.15 0.15 0.5] get value
      (for _array_element (Variables|Default|GetSlots)
        (bind _asbp_button_padlock_num (Utilities|Casting|CastToBP_Button_padlock_num _array_element))
        (Utilities|Array|Add _pattern (Variables|/Game/Blueprints/Locks/BP_Button_padlock_num.BP_Button_padlock_num_C|GetValue _asbp_button_padlock_num))
        ;[0.15 0.15 0.15 0.5] compare
        (Utilities|FlowControl|Delay 0.2)
        (if (Utilities|Array|Identical (Variables|Default|GetCorrectPattern) _pattern)
          ;[0.15 0.15 0.15 0.5] hologram removal
          (bind _outactors (Actor|GetAllActorsOfClass "/Game/Blueprints/Locks/BP_Button_padlock_num.BP_Button_padlock_num_C"))
          (for (_array_element_2 _array_index) _outactors
            (if (<= _array_index 4)
              (Default|DestroyNumbers _array_element_2)
              (Variables|Default|SetEnd true)))
          (else
            (Utilities|Array|Clear _pattern))))
      (else
        ;[0.15 0.15 0.15 0.5] Spawning Numbers
        (for (_array_element_3 _array_index_2) (Variables|Default|GetSlots)
          (Transformation|Teleport _array_element_3 (- (Transformation|GetWorldLocation _padlock) (Utilities|Array|Get(acopy) (Variables|Default|GetLocation) _array_index_2)) (Transformation|GetWorldRotation _padlock)))
        (Variables|Default|SetIs_Spawned true)))))

(fn ConstructionScript)