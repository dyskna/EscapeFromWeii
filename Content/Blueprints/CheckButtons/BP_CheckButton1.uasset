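; Check button for a two-stage button puzzle, triggered by overlap and animated with a Timeline that presses and releases it.
; On release, stage one (Etap) matches BP_Button pressed states to a pattern; stage two also requires the press order recorded via RegisterClicked.
; Success flashes the button green, blacks out the directional light, swaps board materials, restores light, then advances or ends the puzzle.
; A failed stage-two check clears the recorded order.
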(event OnComponentBeginOverlap(Box)
  (params (OverlappedComponent :type Primitive%20Component%20Object%20Reference) (OtherActor :type Actor%20Object%20Reference) (OtherComp :type Primitive%20Component%20Object%20Reference) (OtherBodyIndex :type Integer) (bFromSweep :type Boolean) (SweepResult :type Hit%20Result%20Structure%20%28by%20ref%29))
  (bind _etap1buttonsstate (Variables|Default|GetEtap1ButtonsState))
  (bind _etap2buttonorder (Variables|Default|GetEtap2ButtonOrder))
  (bind _etap1buttonsstate_2 (Variables|Default|GetEtap1ButtonsState))
  (bind _button (Variables|Default|GetButton))
  ;[0.15 0.15 0.15 0.5] Button press animation
  (if (not (Variables|Default|GetIsClicked))
    (Variables|Default|SetIsClicked true)
    (Collision|SetCollisionEnabled _button "NoCollision")
    (bind _alpha (Timeline|Timeline Play)
      (:Update
        (Transformation|SetRelativeLocation (Variables|Default|GetButton) (Math|Vector|Lerp(Vector) "0, 0, 0" "0.000000,-3.000000,0.000000" _alpha) false false))
      (:Finished
        (if (Variables|Default|GetIsClicked)
          (Variables|Default|SetIsClicked false)
          (Timeline|Timeline Reverse)
          (else
            (Collision|SetCollisionEnabled _button "QueryAndPhysics")
            (if (not (Variables|Default|GetEnd))
              (if (Variables|Default|GetEtap)
                ;[0.15 0.15 0.15 0.5] Checking state of buttons
                (for (_array_element _array_index) (Variables|Default|GetButtons)
                  (bind _asbp_button (Utilities|Casting|CastToBP_Button _array_element))
                  (Utilities|Array|SetArrayElem _etap1buttonsstate _array_index (Variables|/Game/Blueprints/BP_Button.BP_Button_C|GetIsPressed _asbp_button)))
                (if (Utilities|Array|Identical (Variables|Default|GetEtap1CorrectPattern) _etap1buttonsstate)
                  ;[0.15 0.15 0.15 0.5] light management
                  (Rendering|Material|SetMaterial (Variables|Default|GetButton) 0 "/Game/VRTemplate/Materials/M_Green.M_Green" :!label _label)
                  (Utilities|FlowControl|Delay 0.1)
                  (bind _asdirectional_light (Utilities|Casting|CastToDirectionalLight (Variables|Default|Getlight)))
                  (Rendering|Components|Light|SetIntensity (Variables|/Script/Engine.Light|GetLightComponent _asdirectional_light) 0.0)
                  (Utilities|FlowControl|Delay 2.0)
                  (Rendering|Material|SetMaterial (Variables|Default|GetButton) 0 "/Game/VRTemplate/Materials/M_Red.M_Red")
                  (if (Variables|Default|GetEtap)
                    ;[0.15 0.15 0.15 0.5] change of environment
                    (bind _asstatic_mesh_actor (Utilities|Casting|CastToStaticMeshActor (Variables|Default|GetChalkBoard)))
                    (Rendering|Material|SetMaterial (Variables|/Script/Engine.StaticMeshActor|GetStaticMeshComponent _asstatic_mesh_actor) 0 "/Game/AssetsWeii/RoomBuild/Furniture/Chalkboard/M_chalkboard2.M_chalkboard2")
                    (bind _asstatic_mesh_actor_2 (Utilities|Casting|CastToStaticMeshActor (Variables|Default|GetWhiteBoard)))
                    (Rendering|Material|SetMaterial (Variables|/Script/Engine.StaticMeshActor|GetStaticMeshComponent _asstatic_mesh_actor_2) 0 "/Game/AssetsWeii/RoomBuild/Furniture/Whiteboard/M_Whiteboard1.M_Whiteboard1")
                    (else
                      ;[0.15 0.15 0.15 0.5] change of environment
                      (bind _asstatic_mesh_actor_3 (Utilities|Casting|CastToStaticMeshActor (Variables|Default|GetChalkBoard)))
                      (Rendering|Material|SetMaterial (Variables|/Script/Engine.StaticMeshActor|GetStaticMeshComponent _asstatic_mesh_actor_3) 0 "/Game/AssetsWeii/RoomBuild/Furniture/Chalkboard/M_chalkboard3.M_chalkboard3")
                      (Variables|Default|SetEnd true)))
                  ;[0.15 0.15 0.15 0.5] light management
                  (bind _asdirectional_light_2 (Utilities|Casting|CastToDirectionalLight (Variables|Default|Getlight)))
                  (Rendering|Components|Light|SetIntensity (Variables|/Script/Engine.Light|GetLightComponent _asdirectional_light_2) 14.0)
                  (Utilities|Array|Clear (Variables|Default|GetEtap2ButtonOrder))
                  (Variables|Default|SetEtap false))
                (else
                  ;[0.15 0.15 0.15 0.5] Checking order of buttons
                  (if (Utilities|Array|Identical (Variables|Default|GetEtap2CorrectButtonOrder) _etap2buttonorder)
                    ;[0.15 0.15 0.15 0.5] Checking state of buttons
                    (for (_array_element_2 _array_index_2) (Variables|Default|GetButtons)
                      (bind _asbp_button_2 (Utilities|Casting|CastToBP_Button _array_element_2))
                      (Utilities|Array|SetArrayElem _etap1buttonsstate_2 _array_index_2 (Variables|/Game/Blueprints/BP_Button.BP_Button_C|GetIsPressed _asbp_button_2)))
                    (if (Utilities|Array|Identical (Variables|Default|GetEtap2CorrectPatern) _etap1buttonsstate_2)
                      (goto _label)
                      (else
                        (Utilities|Array|Clear (Variables|Default|GetEtap2ButtonOrder))))
                    (else
                      (Utilities|Array|Clear _etap2buttonorder))))))))))))

(fn ConstructionScript)

(fn RegisterClicked
  (params (ButtonID :type Integer))
  (Utilities|Array|Add (Variables|Default|GetEtap2ButtonOrder) ButtonID))