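; Pickable VR card actor that can be grabbed by hand and slid along with a drawer as it opens.
; On grab and drop, its grab snap component toggles move-ignore and player input, and hides or restores that hand's message on the motion controller's owner, avoiding a hard VR pawn reference.
; MoveCard uses a timeline to lerp the root from its starting location by a supplied offset.
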(event OnGrabbed(GrabComponentSnap)
  (bind _grabcomponentsnap (Variables|Default|GetGrabComponentSnap))
  (Development|PrintString "CARD GRABBED")
  (Collision|IgnoreActorwhenMoving (Variables|Default|GetCard) 0 true)
  (Input|EnableInput (Game|GetPlayerController 0))
  (Class|BPIPawnAnim|HideUnhideHand(Message) (Components|GetOwner (Variables|/Game/VRTemplate/Blueprints/GrabComponent.GrabComponent_C|GetMotionControllerRef _grabcomponentsnap)) true (Utilities|Enum|Equal(Enum) (Default|GetHeldbyHand _grabcomponentsnap) "Right")))

(event OnDropped(GrabComponentSnap)
  (bind _grabcomponentsnap (Variables|Default|GetGrabComponentSnap))
  (Development|PrintString "CARD DROPPED")
  (Collision|IgnoreActorwhenMoving (Variables|Default|GetCard) 0 false)
  (Input|DisableInput (Game|GetPlayerController 0))
  (Class|BPIPawnAnim|HideUnhideHand(Message) (Components|GetOwner (Variables|/Game/VRTemplate/Blueprints/GrabComponent.GrabComponent_C|GetMotionControllerRef _grabcomponentsnap)) false (Utilities|Enum|Equal(Enum) (Default|GetHeldbyHand _grabcomponentsnap) "Right")))

(event Custom|MoveCard
  (params (OpenOffset :type Vector))
  ;[0.15 0.15 0.15 0.5] Move the card with the drawer when it opens
  (Variables|Default|SetOriginalCardLocation (Transformation|GetWorldLocation (Variables|Default|GetDefaultSceneRoot)))
  (bind _alpha (Timeline|Timeline Play)
    (:Update
      (Transformation|SetRelativeLocation (Variables|Default|GetDefaultSceneRoot) (Math|Vector|Lerp(Vector) (Variables|Default|GetOriginalCardLocation) (+ (Variables|Default|GetOriginalCardLocation) OpenOffset) _alpha) false false))))

(fn ConstructionScript)