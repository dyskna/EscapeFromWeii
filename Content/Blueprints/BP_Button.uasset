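; BP_Button is a pressable button that reports its ButtonID to BP_CheckButton1 when something overlaps its collision component.
; On each begin overlap it finds the BP_CheckButton1 actors with GetAllActorsOfClass and calls RegisterClicked on them.
; It then toggles IsPressed and plays or reverses a timeline that lerps the Button component down along Z, so a second overlap raises it again.
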(event OnComponentBeginOverlap(ButtonColision)
  (params (OverlappedComponent :type Primitive%20Component%20Object%20Reference) (OtherActor :type Actor%20Object%20Reference) (OtherComp :type Primitive%20Component%20Object%20Reference) (OtherBodyIndex :type Integer) (bFromSweep :type Boolean) (SweepResult :type Hit%20Result%20Structure%20%28by%20ref%29))
  (bind _outactors (Actor|GetAllActorsOfClass "/Game/Blueprints/BP_CheckButton1.BP_CheckButton1_C"))
  (Default|RegisterClicked _outactors (Variables|Default|GetButtonID))
  ;[0.15 0.15 0.15 0.5] Button press animation
  (if (Variables|Default|GetIsPressed)
    (Variables|Default|SetIsPressed false)
    (bind _alpha (Timeline|Timeline_0 Reverse)
      (:Update
        (Transformation|SetRelativeLocation (Variables|Default|GetButton) (Math|Vector|Lerp(Vector) "0, 0, 0" "0.000000,0.000000,-55.000000" _alpha) false false)))
    (else
      (Variables|Default|SetIsPressed true)
      (Timeline|Timeline_0 Play))))

(fn ConstructionScript)