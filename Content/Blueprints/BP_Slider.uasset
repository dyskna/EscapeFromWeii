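; BP_Slider is an overlap-triggered puzzle button that toggles between raised and pressed via a timeline, with collision disabled while it moves.
; When the animation finishes, it registers its ButtonID with BP_CheckButton1 if that checker's Etap flag is false.
; At six entries, a correct order blacks out the directional light while the chalkboard switches to the third riddle.
; A wrong order clears the list and reverses all pressed sliders, using ReverseEnd to suppress re-registration.
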(event OnComponentBeginOverlap(ButtonColision)
  (params (OverlappedComponent :type Primitive%20Component%20Object%20Reference) (OtherActor :type Actor%20Object%20Reference) (OtherComp :type Primitive%20Component%20Object%20Reference) (OtherBodyIndex :type Integer) (bFromSweep :type Boolean) (SweepResult :type Hit%20Result%20Structure%20%28by%20ref%29))
  (Variables|Default|SetReverseEnd false)
  ;[0.15 0.15 0.15 0.5] Button press animation
  (Collision|SetCollisionEnabled (Variables|Collision|GetButtonColision) "NoCollision")
  (if (Variables|Default|GetIsPressed)
    (Variables|Default|SetIsPressed false)
    (bind _alpha (Timeline|Timeline Reverse)
      (:Update
        (Transformation|SetRelativeLocation (Variables|Default|GetButton) (Math|Vector|Lerp(Vector) "0, 0, 0" "0.000000,0.000000,-40.000000" _alpha) false false))
      (:Finished
        (if (not (Variables|Default|GetReverseEnd))
          (Collision|SetCollisionEnabled (Variables|Collision|GetButtonColision) "QueryAndPhysics")
          (bind _asbp_check_button_1 (Utilities|Casting|CastToBP_CheckButton1 (Variables|Default|GetBP_CheckButton1)))
          (if (not (Variables|/Game/Blueprints/Buttons/BP_CheckButton1.BP_CheckButton1_C|GetEtap _asbp_check_button_1))
            ;[0.15 0.15 0.15 0.5] Checking order of buttons
            (bind _asbp_check_button_1_2 (Utilities|Casting|CastToBP_CheckButton1 (Variables|Default|GetBP_CheckButton1)))
            (Default|RegisterClicked _asbp_check_button_1_2 (Variables|Default|GetButtonID))
            (Development|PrintString (Utilities|String|ToString(Integer) (Utilities|Array|Length (Variables|/Game/Blueprints/Buttons/BP_CheckButton1.BP_CheckButton1_C|GetEtap2ButtonOrder _asbp_check_button_1_2))))
            (if (== (Utilities|Array|Length (Variables|/Game/Blueprints/Buttons/BP_CheckButton1.BP_CheckButton1_C|GetEtap2ButtonOrder _asbp_check_button_1_2)) 6)
              (if (Utilities|Array|Identical (Variables|/Game/Blueprints/Buttons/BP_CheckButton1.BP_CheckButton1_C|GetEtap2ButtonOrder _asbp_check_button_1_2) (Variables|Default|GetTemp))
                ;[0.15 0.15 0.15 0.5] light management
                (Utilities|FlowControl|Delay 0.1)
                (bind _asdirectional_light (Utilities|Casting|CastToDirectionalLight (Variables|Default|Getlight)))
                (Rendering|Components|Light|SetIntensity (Variables|/Script/Engine.Light|GetLightComponent _asdirectional_light) 0.0)
                (Utilities|FlowControl|Delay 2.0)
                ;[0.15 0.15 0.15 0.5] change of environment
                (bind _asstatic_mesh_actor (Utilities|Casting|CastToStaticMeshActor (Variables|Default|GetChalkBoard)))
                (Rendering|Material|SetMaterial (Variables|/Script/Engine.StaticMeshActor|GetStaticMeshComponent _asstatic_mesh_actor) 0 "/Game/AssetsWeii/RoomBuild/Furniture/Boards/Chalkboard/M_ChalkboardRiddle3.M_ChalkboardRiddle3")
                ;[0.15 0.15 0.15 0.5] light management
                (bind _asdirectional_light_2 (Utilities|Casting|CastToDirectionalLight (Variables|Default|Getlight)))
                (Rendering|Components|Light|SetIntensity (Variables|/Script/Engine.Light|GetLightComponent _asdirectional_light_2) 14.0)
                (else
                  (Utilities|Array|Clear (Variables|/Game/Blueprints/Buttons/BP_CheckButton1.BP_CheckButton1_C|GetEtap2ButtonOrder _asbp_check_button_1_2))
                  (for _array_element (Variables|Default|GetSlidersRef)
                    (if (Variables|BP_Slider_C|GetIsPressed _array_element)
                      (Variables|BP_Slider_C|SetIsPressed _array_element false)
                      (CallFunction|ReversefromEnd _array_element))))))))))
    (else
      (Variables|Default|SetIsPressed true)
      (Timeline|Timeline Play))))

(event Custom|Animation
  ;[0.15 0.15 0.15 0.5] Button press animation
  (Collision|SetCollisionEnabled (Variables|Collision|GetButtonColision) "NoCollision")
  (if (Variables|Default|GetIsPressed)
    (Variables|Default|SetIsPressed false)
    (bind _alpha (Timeline|Timeline_0 Reverse)
      (:Update
        (Transformation|SetRelativeLocation (Variables|Default|GetButton) (Math|Vector|Lerp(Vector) "0, 0, 0" "0.000000,0.000000,-40.000000" _alpha) false false))
      (:Finished
        (Collision|SetCollisionEnabled (Variables|Collision|GetButtonColision) "QueryAndPhysics")))
    (else
      (Variables|Default|SetIsPressed true)
      (Timeline|Timeline_0 Play))))

(event Custom|ReverseFromEnd
  ;[0.15 0.15 0.15 0.5] Button press animation
  (Variables|Default|SetReverseEnd true)
  (bind _alpha (Timeline|Timeline ReverseFromEnd)
    (:Update
      (Transformation|SetRelativeLocation (Variables|Default|GetButton) (Math|Vector|Lerp(Vector) "0, 0, 0" "0.000000,0.000000,-40.000000" _alpha) false false))
    (:Finished
      (if (not (Variables|Default|GetReverseEnd))
        (Collision|SetCollisionEnabled (Variables|Collision|GetButtonColision) "QueryAndPhysics")
        (bind _asbp_check_button_1 (Utilities|Casting|CastToBP_CheckButton1 (Variables|Default|GetBP_CheckButton1)))
        (if (not (Variables|/Game/Blueprints/Buttons/BP_CheckButton1.BP_CheckButton1_C|GetEtap _asbp_check_button_1))
          ;[0.15 0.15 0.15 0.5] Checking order of buttons
          (bind _asbp_check_button_1_2 (Utilities|Casting|CastToBP_CheckButton1 (Variables|Default|GetBP_CheckButton1)))
          (Default|RegisterClicked _asbp_check_button_1_2 (Variables|Default|GetButtonID))
          (Development|PrintString (Utilities|String|ToString(Integer) (Utilities|Array|Length (Variables|/Game/Blueprints/Buttons/BP_CheckButton1.BP_CheckButton1_C|GetEtap2ButtonOrder _asbp_check_button_1_2))))
          (if (== (Utilities|Array|Length (Variables|/Game/Blueprints/Buttons/BP_CheckButton1.BP_CheckButton1_C|GetEtap2ButtonOrder _asbp_check_button_1_2)) 6)
            (if (Utilities|Array|Identical (Variables|/Game/Blueprints/Buttons/BP_CheckButton1.BP_CheckButton1_C|GetEtap2ButtonOrder _asbp_check_button_1_2) (Variables|Default|GetTemp))
              ;[0.15 0.15 0.15 0.5] light management
              (Utilities|FlowControl|Delay 0.1)
              (bind _asdirectional_light (Utilities|Casting|CastToDirectionalLight (Variables|Default|Getlight)))
              (Rendering|Components|Light|SetIntensity (Variables|/Script/Engine.Light|GetLightComponent _asdirectional_light) 0.0)
              (Utilities|FlowControl|Delay 2.0)
              ;[0.15 0.15 0.15 0.5] change of environment
              (bind _asstatic_mesh_actor (Utilities|Casting|CastToStaticMeshActor (Variables|Default|GetChalkBoard)))
              (Rendering|Material|SetMaterial (Variables|/Script/Engine.StaticMeshActor|GetStaticMeshComponent _asstatic_mesh_actor) 0 "/Game/AssetsWeii/RoomBuild/Furniture/Boards/Chalkboard/M_ChalkboardRiddle3.M_ChalkboardRiddle3")
              ;[0.15 0.15 0.15 0.5] light management
              (bind _asdirectional_light_2 (Utilities|Casting|CastToDirectionalLight (Variables|Default|Getlight)))
              (Rendering|Components|Light|SetIntensity (Variables|/Script/Engine.Light|GetLightComponent _asdirectional_light_2) 14.0)
              (else
                (Utilities|Array|Clear (Variables|/Game/Blueprints/Buttons/BP_CheckButton1.BP_CheckButton1_C|GetEtap2ButtonOrder _asbp_check_button_1_2))
                (for _array_element (Variables|Default|GetSlidersRef)
                  (if (Variables|BP_Slider_C|GetIsPressed _array_element)
                    (Variables|BP_Slider_C|SetIsPressed _array_element false)
                    (CallFunction|ReversefromEnd _array_element)))))))))))

(fn ConstructionScript)