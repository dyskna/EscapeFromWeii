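; Card scanner and keypad puzzle that opens the Asseco level once three diodes are lit green.
; Keypad input builds a code of up to four digits shown through screen materials, and two distinct codes can each light a diode once.
; A card swipe must overlap four trigger volumes top to bottom within timed windows to light another.
; Failed codes or swipes briefly flash the next diode red.
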(event OnComponentBeginOverlap(ScannerTop)
  (params (OverlappedComponent :type Primitive%20Component%20Object%20Reference) (OtherActor :type Actor%20Object%20Reference) (OtherComp :type Primitive%20Component%20Object%20Reference) (OtherBodyIndex :type Integer) (bFromSweep :type Boolean) (SweepResult :type Hit%20Result%20Structure%20%28by%20ref%29))
  ;[0.15 0.15 0.15 0.5] Card scanning
  (if (and (== OtherActor (Variables|Default|GetCardRef)) (!= (Variables|Default|GetCardProgress) 4))
    (Development|PrintString "Top")
    (Variables|Default|SetCardProgress 1)
    (Variables|Default|SetTopScanned true)
    (Utilities|FlowControl|Delay (Variables|Default|GetScanTime))
    (Variables|Default|SetTopScanned false)))

(event OnComponentBeginOverlap(ScannerMiddleTop)
  (params (OverlappedComponent :type Primitive%20Component%20Object%20Reference) (OtherActor :type Actor%20Object%20Reference) (OtherComp :type Primitive%20Component%20Object%20Reference) (OtherBodyIndex :type Integer) (bFromSweep :type Boolean) (SweepResult :type Hit%20Result%20Structure%20%28by%20ref%29))
  ;[0.15 0.15 0.15 0.5] Card scanning
  (if (and (== OtherActor (Variables|Default|GetCardRef)) (!= (Variables|Default|GetCardProgress) 4))
    (Development|PrintString "MiddleTop")
    (if (and (== (Variables|Default|GetCardProgress) 1) (Variables|Default|GetTopScanned))
      (Variables|Default|SetCardProgress 2)
      (Variables|Default|SetMiddleTopScanned true)
      (Utilities|FlowControl|Delay (Variables|Default|GetScanTime))
      (Variables|Default|SetMiddleTopScanned false)
      (else
        (CallFunction|RedDiode)))))

(event OnComponentBeginOverlap(ScannerMiddleBottom)
  (params (OverlappedComponent :type Primitive%20Component%20Object%20Reference) (OtherActor :type Actor%20Object%20Reference) (OtherComp :type Primitive%20Component%20Object%20Reference) (OtherBodyIndex :type Integer) (bFromSweep :type Boolean) (SweepResult :type Hit%20Result%20Structure%20%28by%20ref%29))
  ;[0.15 0.15 0.15 0.5] Card scanning
  (if (and (== OtherActor (Variables|Default|GetCardRef)) (!= (Variables|Default|GetCardProgress) 4))
    (Development|PrintString "MiddleBottom")
    (if (and (== (Variables|Default|GetCardProgress) 2) (Variables|Default|GetMiddleTopScanned))
      (Variables|Default|SetCardProgress 3)
      (Variables|Default|SetMiddleBottomScanned true)
      (Utilities|FlowControl|Delay (Variables|Default|GetScanTime))
      (Variables|Default|SetMiddleBottomScanned false)
      (else
        (CallFunction|RedDiode)))))

(event OnComponentBeginOverlap(ScannerBottom)
  (params (OverlappedComponent :type Primitive%20Component%20Object%20Reference) (OtherActor :type Actor%20Object%20Reference) (OtherComp :type Primitive%20Component%20Object%20Reference) (OtherBodyIndex :type Integer) (bFromSweep :type Boolean) (SweepResult :type Hit%20Result%20Structure%20%28by%20ref%29))
  ;[0.15 0.15 0.15 0.5] Card scanning
  (if (and (== OtherActor (Variables|Default|GetCardRef)) (!= (Variables|Default|GetCardProgress) 4))
    (Development|PrintString "Bottom")
    (if (and (== (Variables|Default|GetCardProgress) 3) (Variables|Default|GetMiddleBottomScanned))
      (Variables|Default|SetCardProgress 4)
      (CallFunction|GreenDiode)
      (else
        (CallFunction|RedDiode)))))

(event Custom|AddDigit
  (params (Digit :type Integer))
  ;[0.15 0.15 0.15 0.5] Add digit to input code
  (if (< (Utilities|Array|Length (Variables|Default|GetInputCode)) 4)
    (Utilities|Array|Add (Variables|Default|GetInputCode) Digit)
    (CallFunction|UpdateScreen)))

(event Custom|RemoveDigit
  (bind _inputcode (Variables|Default|GetInputCode))
  ;[0.15 0.15 0.15 0.5] Remove last digit from input code
  (if (!= (Utilities|Array|Length (Variables|Default|GetInputCode)) 0)
    (Utilities|Array|RemoveIndex _inputcode (Utilities|Array|LastIndex _inputcode))
    (CallFunction|UpdateScreen)))

(event Custom|CheckCode
  (bind _inputcode (Variables|Default|GetInputCode))
  ;[0.15 0.15 0.15 0.5] Check if input code is correct
  (if (Utilities|Array|Identical (Variables|Default|GetCorrectCode1) _inputcode)
    (if (not (Variables|Default|GetDoneCorrectCode1))
      (Variables|Default|SetDoneCorrectCode1 true)
      (Development|PrintString "Correct Code 1")
      (Utilities|Array|Clear (Variables|Default|GetInputCode) :!label _label)
      (CallFunction|GreenDiode))
    (elif (Utilities|Array|Identical _inputcode (Variables|Default|GetCorrectCode2))
      (if (not (Variables|Default|GetDoneCorrectCode2))
        (Variables|Default|SetDoneCorrectCode2 true)
        (Development|PrintString "Correct Code 2")
        (goto _label))
      (else
        (Utilities|Array|Clear (Variables|Default|GetInputCode))
        (CallFunction|RedDiode)
        (CallFunction|UpdateScreen)))))

(event Custom|GreenDiode
  ;[0.15 0.15 0.15 0.5] Light a green diode
  (bind _output_get (Variables|Default|SetDiodeCounter (+ (Variables|Default|GetDiodeCounter) 1)))
  (switch int _output_get
    (:1
      (bind _output_get_2 (Variables|Default|SetTargetDiode (Variables|Default|GetDiode1Ref))))
    (:2
      (bind _output_get_3 (Variables|Default|SetTargetDiode (Variables|Default|GetDiode2Ref))))
    (:3
      (bind _output_get_4 (Variables|Default|SetTargetDiode (Variables|Default|GetDiode3Ref)))))
  (Rendering|Material|SetMaterial (Variables|/Game/Blueprints/CardScanner/Diode.Diode_C|GetCardScanner _output_get_3) 1 "/Game/AssetsWeii/RoomBuild/Electronics/Diode/M_DiodeGreenON.M_DiodeGreenON")
  (CallFunction|PuzzleCompleted))

(event Custom|RedDiode
  ;[0.15 0.15 0.15 0.5] Light a red diode
  (switch int (Variables|Default|GetDiodeCounter)
    (:0
      (bind _output_get (Variables|Default|SetTargetDiode (Variables|Default|GetDiode1Ref))))
    (:1
      (bind _output_get_2 (Variables|Default|SetTargetDiode (Variables|Default|GetDiode2Ref))))
    (:2
      (bind _output_get_3 (Variables|Default|SetTargetDiode (Variables|Default|GetDiode3Ref)))))
  (Rendering|Material|SetMaterial (Variables|/Game/Blueprints/CardScanner/Diode.Diode_C|GetCardScanner _output_get) 1 "/Game/AssetsWeii/RoomBuild/Electronics/Diode/M_DiodeRedON.M_DiodeRedON")
  (Utilities|FlowControl|Delay 1.0)
  (if (== (Rendering|Material|GetMaterial (Variables|/Game/Blueprints/CardScanner/Diode.Diode_C|GetCardScanner _output_get_2) 1) "/Game/AssetsWeii/RoomBuild/Electronics/Diode/M_DiodeRedON.M_DiodeRedON")
    (Rendering|Material|SetMaterial (Variables|/Game/Blueprints/CardScanner/Diode.Diode_C|GetCardScanner _output_get_3) 1 "/Game/AssetsWeii/RoomBuild/Electronics/Diode/M_DiodeRedOFF.M_DiodeRedOFF")))

(event Custom|UpdateScreen
  (bind _screenref (Variables|Default|GetScreenRef))
  (bind _cardscanner (Variables|/Game/Blueprints/CardScanner/Screen.Screen_C|GetCardScanner _screenref))
  ;[0.15 0.15 0.15 0.5] Update screen material
  (switch int (Utilities|Array|Length (Variables|Default|GetInputCode))
    (:0
      (Rendering|Material|SetMaterial _cardscanner 1 "/Game/AssetsWeii/RoomBuild/Riddles/Keypad/M_KeypadScreen.M_KeypadScreen"))
    (:1
      (Rendering|Material|SetMaterial _cardscanner 1 "/Game/AssetsWeii/RoomBuild/Riddles/Keypad/M_KeypadScreen1.M_KeypadScreen1") ; Change material to "*"
    )
    (:2
      (Rendering|Material|SetMaterial _cardscanner 1 "/Game/AssetsWeii/RoomBuild/Riddles/Keypad/M_KeypadScreen2.M_KeypadScreen2") ; Change material to "**"
    )
    (:3
      (Rendering|Material|SetMaterial _cardscanner 1 "/Game/AssetsWeii/RoomBuild/Riddles/Keypad/M_KeypadScreen3.M_KeypadScreen3") ; Change material to "***"
    )
    (:4
      (Rendering|Material|SetMaterial _cardscanner 1 "/Game/AssetsWeii/RoomBuild/Riddles/Keypad/M_KeypadScreen4.M_KeypadScreen4") ; Change material to "****"
    )))

(event Custom|PuzzleCompleted
  ;[0.15 0.15 0.15 0.5] Completing the puzzle
  (if (== (Variables|Default|GetDiodeCounter) 3)
    (Game|OpenLevel(byObjectReference) "/Game/Asseco.Asseco")))

(fn ConstructionScript)