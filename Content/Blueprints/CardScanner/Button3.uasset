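; Button3 is a card scanner keypad button that enters the digit 3 when an actor overlaps it.
; An overlap disables the button mesh's collision and plays a Timeline that lerps it inward along X, then reverses it.
; Once the return finishes, collision is restored and the digit is sent to the referenced CardScanner via AddDigit.
; The IsPressed flag blocks re-triggering during the press and tells the Finished handler which direction just completed.
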(event Collision|EventActorBeginOverlap
  (params (OtherActor :type Actor%20Object%20Reference))
  (bind _button3 (Variables|Default|GetButton3))
  ;[0.15 0.15 0.15 0.5] Button press (logic and animation)
  (if (not (Variables|Default|GetIsPressed))
    (Variables|Default|SetIsPressed true)
    (Collision|SetCollisionEnabled _button3 "NoCollision")
    (bind _alpha (Timeline|Timeline Play)
      (:Update
        (Transformation|SetRelativeLocation (Variables|Default|GetButton3) (Math|Vector|Lerp(Vector) "0, 0, 0" "-3.000000,0.000000,0.000000" _alpha) false false))
      (:Finished
        (if (Variables|Default|GetIsPressed)
          (Variables|Default|SetIsPressed false)
          (Timeline|Timeline Reverse)
          (else
            (Collision|SetCollisionEnabled _button3 "QueryAndPhysics")
            ;[0.15 0.15 0.15 0.5] Add digit to input code
            (Default|AddDigit (Variables|Default|GetCardScannerRef) 3)))))))

(fn ConstructionScript)