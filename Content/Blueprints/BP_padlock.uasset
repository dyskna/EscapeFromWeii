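; BP_padlock is a padlock actor that creates its row of number buttons when something first overlaps its Box trigger.
; The overlap spawns five BP_Button_padlock actors, evenly spaced along world X and raised above the Padlock component's location, ignoring its rotation.
; An IsSpawned flag prevents repeat spawning, and the spawned buttons are not stored or wired back to the padlock.
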(event OnComponentBeginOverlap(Box)
  (params (OverlappedComponent :type Primitive%20Component%20Object%20Reference) (OtherActor :type Actor%20Object%20Reference) (OtherComp :type Primitive%20Component%20Object%20Reference) (OtherBodyIndex :type Integer) (bFromSweep :type Boolean) (SweepResult :type Hit%20Result%20Structure%20%28by%20ref%29))
  (bind _padlock (Variables|Default|Getpadlock))
  (bind _returnvalue (Transformation|GetWorldLocation _padlock))
  (if (not (Variables|Default|GetIs_Spawned))
    ;[0.15 0.15 0.15 0.5] Spawning Numbers
    (Game|SpawnActorfromClass "/Game/Blueprints/BP_Button_padlock.BP_Button_padlock_C" (Math|Transform|MakeTransform (- _returnvalue "28.000000,0.000000,-30.000000") "0, 0, 0" "1.000000,1.000000,1.000000") "Undefined" "MultiplyWithRoot" 0 0 0)
    (Game|SpawnActorfromClass "/Game/Blueprints/BP_Button_padlock.BP_Button_padlock_C" (Math|Transform|MakeTransform (- _returnvalue "14.000000,0.000000,-30.000000") "0, 0, 0" "1.000000,1.000000,1.000000") "Undefined" "MultiplyWithRoot" 0 0 0)
    (Game|SpawnActorfromClass "/Game/Blueprints/BP_Button_padlock.BP_Button_padlock_C" (Math|Transform|MakeTransform (- _returnvalue "0.000000,0.000000,-30.000000") "0, 0, 0" "1.000000,1.000000,1.000000") "Undefined" "MultiplyWithRoot" 0 0 0)
    (Game|SpawnActorfromClass "/Game/Blueprints/BP_Button_padlock.BP_Button_padlock_C" (Math|Transform|MakeTransform (- _returnvalue "-14.000000,0.000000,-30.000000") "0, 0, 0" "1.000000,1.000000,1.000000") "Undefined" "MultiplyWithRoot" 0 0 0)
    (Game|SpawnActorfromClass "/Game/Blueprints/BP_Button_padlock.BP_Button_padlock_C" (Math|Transform|MakeTransform (- _returnvalue "-28.000000,0.000000,-30.000000") "0, 0, 0" "1.000000,1.000000,1.000000") "Undefined" "MultiplyWithRoot" 0 0 0)
    (Variables|Default|SetIs_Spawned true)))

(fn ConstructionScript)