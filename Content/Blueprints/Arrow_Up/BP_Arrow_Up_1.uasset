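; BP_Arrow_Up_1 is an up-arrow trigger that steps a single digit Value from 0 to 9 when something overlaps its Box.
; Wrapping past 9 resets Value and spawns a Num_0_0 actor below the Arrow without storing it.
; Other increments either spawn and store that actor in Slot1 or destroy Slot1, depending on Num0.
; The logic deriving Num0 and Num1 from Value is unconnected and never runs.
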(event OnComponentBeginOverlap(Box)
  (params (OverlappedComponent :type Primitive%20Component%20Object%20Reference) (OtherActor :type Actor%20Object%20Reference) (OtherComp :type Primitive%20Component%20Object%20Reference) (OtherBodyIndex :type Integer) (bFromSweep :type Boolean) (SweepResult :type Hit%20Result%20Structure%20%28by%20ref%29))
  (if (> (+ (Variables|Default|Getvalue) 1) 9)
    (Variables|Default|Setvalue 0)
    (Game|SpawnActorfromClass "/Game/Blueprints/Numbers/Num_0_0.Num_0_0_C" (Math|Transform|MakeTransform (- (Transformation|GetWorldLocation (Variables|Default|GetArrow)) "0.000000,0.000000,36.000000") "0, 0, 0" "1.000000,1.000000,1.000000") "Undefined" "MultiplyWithRoot" 0 0)
    (else
      (bind _output_get (Variables|Default|Setvalue (+ (Variables|Default|Getvalue) 1)))
      (if (Variables|Default|GetNum_0)
        (bind _returnvalue (Game|SpawnActorfromClass "/Game/Blueprints/Numbers/Num_0_0.Num_0_0_C" (Math|Transform|MakeTransform (- (Transformation|GetWorldLocation (Variables|Default|GetArrow)) "0.000000,0.000000,36.000000") "0, 0, 0" "1.000000,1.000000,1.000000") "Undefined" "MultiplyWithRoot" 0 0))
        (Variables|Default|SetSlot_1 _returnvalue)
        (else
          (Actor|DestroyActor (Variables|Default|GetSlot_1)))))))

(fn ConstructionScript)