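; Trigger volume inside the elevator that ends the game when its box is overlapped.
; While its Active flag is set, the first overlap clears it, closes the referenced left and right doors, and enables collision on a separate invisible wall actor.
; After a short delay it only prints an end-of-game message.
; The overlap does not check which actor entered.
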(event OnComponentBeginOverlap(Box)
  (params (OverlappedComponent :type Primitive%20Component%20Object%20Reference) (OtherActor :type Actor%20Object%20Reference) (OtherComp :type Primitive%20Component%20Object%20Reference) (OtherBodyIndex :type Integer) (bFromSweep :type Boolean) (SweepResult :type Hit%20Result%20Structure%20%28by%20ref%29))
  ;[0.15 0.15 0.15 0.5] Elevator door closing and game end logic
  (if (Variables|Default|GetActive)
    (Variables|Default|SetActive false)
    (Default|CloseElevatorLeft (Variables|References|GetElevatorDoorLeftRef))
    (Default|CloseElevatorRight (Variables|References|GetElevatorDoorRightRef))
    (Collision|SetCollisionEnabled (Variables|/Game/Blueprints/Elevator/BP_elevator_invisible_collision.BP_elevator_invisible_collision_C|GetWall (Variables|References|GetElevatorInvisibleCollisionRef)) "QueryAndPhysics")
    (Utilities|FlowControl|Delay 1.25)
    (Development|PrintString "THE END OF THE GAME!" true true "(R=0.000000,G=0.660000,B=1.000000,A=1.000000)" 1e+01)))

(fn ConstructionScript)