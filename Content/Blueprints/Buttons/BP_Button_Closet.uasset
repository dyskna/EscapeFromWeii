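; Button that spells out S, H, A, K, E one letter per press by opening groups of BP_Closet actors.
; An overlap plays a press timeline, fires the check at full depression, then reverses, with collision off until the button returns.
; If every closet is closed, a counter selects the next letter's closet array and wraps after E.
; A self-calling event with a short delay opens that letter's closets in sequence.
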(event OnComponentBeginOverlap(Box)
  (params (OverlappedComponent :type Primitive%20Component%20Object%20Reference) (OtherActor :type Actor%20Object%20Reference) (OtherComp :type Primitive%20Component%20Object%20Reference) (OtherBodyIndex :type Integer) (bFromSweep :type Boolean) (SweepResult :type Hit%20Result%20Structure%20%28by%20ref%29))
  (bind _box (Variables|Default|GetBox))
  ;[0.15 0.15 0.15 0.5] Button press animation
  (if (not (Variables|Default|GetIsPressed))
    (Variables|Default|SetIsPressed true)
    (Collision|SetCollisionEnabled _box "NoCollision")
    (bind _alpha (Timeline|Timeline%20Button%20Animation Play)
      (:Update
        (Transformation|SetRelativeLocation (Variables|Default|GetButton) (Math|Vector|Lerp(Vector) "0, 0, 0" "0.000000,-3.000000,0.000000" _alpha) false false))
      (:Finished
        (if (Variables|Default|GetIsPressed)
          (Variables|Default|SetIsPressed false)
          (CallFunction|OnButtonPressed)
          (Timeline|Timeline%20Button%20Animation Reverse)
          (else
            (Collision|SetCollisionEnabled _box "QueryAndPhysics")))))))

(event Custom|OnButtonPressed
  ;[0.15 0.15 0.15 0.5] Checking if all closets are closed
  (Variables|Default|SetBreak false)
  (bind _array_element (Utilities|Array|ForEachLoopwithBreak (Variables|Default|GetAll_Closets) :!label _label)
    (:LoopBody
      (bind _asbp_closet (Utilities|Casting|CastToBP_Closet _array_element))
      (if (Variables|/Game/Blueprints/Closet/BP_Closet.BP_Closet_C|GetIsOpen _asbp_closet)
        (Variables|Default|SetBreak true)
        (goto _label Break)))
    (:Completed
      (if (not (Variables|Default|GetBreak))
        (Utilities|FlowControl|Sequence
          (:then_0
            ;[0.15 0.15 0.15 0.5] Choosing target letter to display based on letter counter
            (switch int (Variables|Default|GetLetter_Counter)
              (:0
                (Variables|Default|SetTarget_Letter (Variables|Default|GetLetter_S)))
              (:1
                (Variables|Default|SetTarget_Letter (Variables|Default|GetLetter_H)))
              (:2
                (Variables|Default|SetTarget_Letter (Variables|Default|GetLetter_A)))
              (:3
                (Variables|Default|SetTarget_Letter (Variables|Default|GetLetter_K)))
              (:4
                (Variables|Default|SetTarget_Letter (Variables|Default|GetLetter_E)))))
          (:then_1
            ;[0.15 0.15 0.15 0.5] Calling event for displaying target letter and incrementing letter counter
            (CallFunction|OpenTargetClosets)
            (if (== (Variables|Default|GetLetter_Counter) 4)
              (Variables|Default|SetLetter_Counter 0)
              (else
                (Variables|Default|SetLetter_Counter (+ (Variables|Default|GetLetter_Counter) 1))))))))))

(event Custom|OpenTargetClosets
  (bind _target_letter (Variables|Default|GetTarget_Letter))
  ;[0.15 0.15 0.15 0.5] Event for displaying target letter
  (if (< (Variables|Default|GetClosetIndex) (Utilities|Array|Length _target_letter))
    (bind _asbp_closet (Utilities|Casting|CastToBP_Closet (Utilities|Array|Get(acopy) _target_letter (Variables|Default|GetClosetIndex))))
    (Default|OpenCloset _asbp_closet)
    (Utilities|FlowControl|Delay 0.2)
    (Variables|Default|SetClosetIndex (+ (Variables|Default|GetClosetIndex) 1))
    (CallFunction|OpenTargetClosets)
    (else
      (Variables|Default|SetClosetIndex 0))))

(fn ConstructionScript)