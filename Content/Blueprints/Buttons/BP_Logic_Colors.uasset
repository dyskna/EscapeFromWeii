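; Logic Blueprint for a Simon-style memory puzzle that drives a set of color buttons, with a placeholder print where an elevator door opening is intended.
; StartColors generates a random color sequence, which the recursive SolutionDisplay flashes up to the current step while button collision is off.
; ColorButtonPressed checks each input, extending the shown sequence on success and completing the puzzle at full length.
; A wrong press triggers Restart, which resets progress and generates a new sequence.
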(event Custom|GlowONAll
  ;[0.15 0.15 0.15 0.5] Events for controlling all color buttons at once
  (for _array_element (Variables|Logic|GetColorButtonsRef)
    (Default|GlowON _array_element)))

(event Custom|PuzzleCompleted
  ;[0.15 0.15 0.15 0.5] Completeing the puzzle
  (CallFunction|DisableCollisionAll)
  (CallFunction|GlowONAll)
  (Development|PrintString "Swap this print for elevator door opening" true true "(R=0.000000,G=0.660000,B=1.000000,A=1.000000)" 1e+01 :!pinned true) ; Swap this print for elevator door opening
)

(event Custom|ColorButtonPressed
  (params (Color :type Integer))
  (bind _input (Variables|Logic|GetInput))
  ;[0.15 0.15 0.15 0.5] Logic for any color button
  (bind _returnvalue (Utilities|Array|Add _input Color))
  (if (!= Color (Utilities|Array|Get(acopy) (Variables|Logic|GetSolution) _returnvalue))
    (CallFunction|Restart)
    (else
      (Collision|SetCollisionEnabled (Variables|/Game/Blueprints/Buttons/BP_Button_Colors.BP_Button_Colors_C|GetCollisionBox (Utilities|Array|Get(acopy) (Variables|Logic|GetColorButtonsRef) Color)) "QueryAndPhysics")
      (if (Utilities|Array|Identical (Variables|Logic|GetInput) (Variables|Logic|GetSolution))
        (CallFunction|PuzzleCompleted)
        (elif (== (Utilities|Array|Length _input) (+ (Variables|Logic|GetStep) 1))
          (Utilities|Array|Clear (Variables|Logic|GetInput))
          (Math|Integer|IncrementInt (Variables|Logic|GetStep)
            (:%20%20
              (Utilities|FlowControl|Delay 0.25)
              (CallFunction|SolutionDisplay))))))))

(event Custom|GenerateSolution
  ;[0.15 0.15 0.15 0.5] Generating a random puzzle solution
  (Utilities|Array|Clear (Variables|Logic|GetSolution))
  (for _index (range 0 (- (Variables|Settings|GetSolutionLength) 1))
    (Utilities|Array|Add (Variables|Logic|GetSolution) (Math|Random|RandomIntegerinRange 0 3))))

(event Custom|EnableCollisionAll
  ;[0.15 0.15 0.15 0.5] Events for controlling all color buttons at once
  (for _array_element (Variables|Logic|GetColorButtonsRef)
    (Collision|SetCollisionEnabled (Variables|/Game/Blueprints/Buttons/BP_Button_Colors.BP_Button_Colors_C|GetCollisionBox _array_element) "QueryAndPhysics")))

(event Custom|Restart
  ;[0.15 0.15 0.15 0.5] Restarting the puzzle
  (Utilities|Array|Clear (Variables|Logic|GetInput))
  (Variables|Logic|SetStep 0)
  (CallFunction|GenerateSolution)
  (CallFunction|GlowONAll)
  (CallFunction|DisableCollisionAll)
  (Utilities|FlowControl|Delay (Variables|Settings|GetRestartGlowTime))
  (CallFunction|GlowOFFAll)
  (CallFunction|EnableCollisionAll)
  (Utilities|FlowControl|Delay (Variables|Settings|GetRestartDelay))
  (CallFunction|SolutionDisplay))

(event Custom|DisableCollisionAll
  ;[0.15 0.15 0.15 0.5] Events for controlling all color buttons at once
  (for _array_element (Variables|Logic|GetColorButtonsRef)
    (Collision|SetCollisionEnabled (Variables|/Game/Blueprints/Buttons/BP_Button_Colors.BP_Button_Colors_C|GetCollisionBox _array_element) "NoCollision")))

(event Custom|SolutionDisplay
  (params (CurrentIndex :type Integer))
  (bind _solution (Variables|Logic|GetSolution))
  (bind _colorbuttonsref (Variables|Logic|GetColorButtonsRef))
  (bind _output (Utilities|Array|Get(acopy) _solution CurrentIndex))
  (bind _output_2 (Utilities|Array|Get(acopy) _colorbuttonsref _output))
  ;[0.15 0.15 0.15 0.5] Displaying the solution step by step
  (if (<= CurrentIndex (Variables|Logic|GetStep))
    (CallFunction|DisableCollisionAll)
    (Default|GlowON _output_2)
    (Utilities|FlowControl|Delay (Variables|Settings|GetSolutionDisplayGlowTime))
    (Default|GlowOFF _output_2)
    (Utilities|FlowControl|Delay (Variables|Settings|GetSolutionDisplayDelay))
    (CallFunction|SolutionDisplay (+ CurrentIndex 1))
    (else
      (CallFunction|EnableCollisionAll))))

(event Custom|GlowOFFAll
  ;[0.15 0.15 0.15 0.5] Events for controlling all color buttons at once
  (for _array_element (Variables|Logic|GetColorButtonsRef)
    (Default|GlowOFF _array_element)))

(event Custom|StartColors
  ;[0.15 0.15 0.15 0.5] Starting the puzzle for the first time
  (CallFunction|GlowOFFAll)
  (CallFunction|EnableCollisionAll)
  (CallFunction|GenerateSolution)
  (Utilities|FlowControl|Delay (Variables|Settings|GetStartDelay))
  (CallFunction|SolutionDisplay))

(event EventBeginPlay
  ;[0.15 0.15 0.15 0.5] Initial (disabled) state of the puzzle
  (CallFunction|GlowONAll)
  (CallFunction|DisableCollisionAll))

(fn ConstructionScript)