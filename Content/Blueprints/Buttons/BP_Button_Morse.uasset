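; BP_Button_Morse is a pressable button that plays a Morse code message from a referenced speaker actor.
; A box overlap disables collision and runs a timeline that pushes the button in and back out.
; On return, collision is restored and a self-calling delayed event plays the letter sounds in sequence.
; Each wait adds three times the Morse "E" sound's duration as a letter gap.
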(event OnComponentBeginOverlap(Box)
  (params (OverlappedComponent :type Primitive%20Component%20Object%20Reference) (OtherActor :type Actor%20Object%20Reference) (OtherComp :type Primitive%20Component%20Object%20Reference) (OtherBodyIndex :type Integer) (bFromSweep :type Boolean) (SweepResult :type Hit%20Result%20Structure%20%28by%20ref%29))
  ;[0.15 0.15 0.15 0.5] Button press (logic and animation)
  (if (not (Variables|Default|GetIsPressed))
    (Variables|Default|SetIsPressed true)
    (Collision|SetCollisionEnabled (Variables|Default|GetBox) "NoCollision")
    (bind _alpha (Timeline|Timeline%20Button%20Animation Play)
      (:Update
        (Transformation|SetRelativeLocation (Variables|Default|GetButton) (Math|Vector|Lerp(Vector) "0, 0, 0" "0.000000,-3.000000,0.000000" _alpha) false false))
      (:Finished
        (if (Variables|Default|GetIsPressed)
          (Variables|Default|SetIsPressed false)
          (Timeline|Timeline%20Button%20Animation Reverse)
          (else
            (CallFunction|LoopwithDelay)
            (Collision|SetCollisionEnabled (Variables|Default|GetBox) "QueryAndPhysics")))))))

(event Custom|LoopWithDelay
  (params (CurrentIndex :type Integer))
  (bind _morselettersref (Variables|Default|GetMorseLettersRef))
  (bind _output (Utilities|Array|Get(acopy) _morselettersref CurrentIndex))
  ;[0.15 0.15 0.15 0.5] Playing the Morse code
  (if (< CurrentIndex (Utilities|Array|Length _morselettersref))
    (Audio|PlaySoundatLocation _output (Transformation|GetActorLocation (Variables|Default|GetSpeakerRef)) "0, 0, 0" 1.0 1.0 0.0 "/Game/Sounds/Attenuation_Speaker.Attenuation_Speaker" 0 0 0)
    (Utilities|FlowControl|Delay (+ (Variables|/Script/Engine.SoundBase|GetDuration _output) (* (Variables|/Script/Engine.SoundBase|GetDuration (Variables|Default|GetEMorseRef)) 3.0)))
    (CallFunction|LoopwithDelay (+ CurrentIndex 1))))

(fn ConstructionScript)