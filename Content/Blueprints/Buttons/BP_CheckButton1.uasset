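; Check button for a slider puzzle that validates the pattern and advances the room to its next riddle.
; Overlapping it plays a press-and-return Timeline, then, while Etap is active, compares BP_Slider states to the correct pattern.
; A match turns it green, blacks out the light, swaps board materials, resets sliders and restores the light.
; RegisterClicked records button IDs for a second stage, which this Blueprint never checks.
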(event OnComponentBeginOverlap(Box)
  (params (OverlappedComponent :type Primitive%20Component%20Object%20Reference) (OtherActor :type Actor%20Object%20Reference) (OtherComp :type Primitive%20Component%20Object%20Reference) (OtherBodyIndex :type Integer) (bFromSweep :type Boolean) (SweepResult :type Hit%20Result%20Structure%20%28by%20ref%29))
  (bind _box (Variables|Default|GetBox))
  (bind _etap1buttonsstate (Variables|Default|GetEtap1ButtonsState))
  ;[0.15 0.15 0.15 0.5] Button press animation
  (if (not (Variables|Default|GetIsClicked))
    (Variables|Default|SetIsClicked true)
    (Collision|SetCollisionEnabled _box "NoCollision")
    (bind _alpha (Timeline|Timeline_0 Play)
      (:Update
        (Transformation|SetRelativeLocation (Variables|Default|GetButton) (Math|Vector|Lerp(Vector) "0, 0, 0" "0.000000,-3.000000,0.000000" _alpha) false false))
      (:Finished
        (if (Variables|Default|GetIsClicked)
          (Variables|Default|SetIsClicked false)
          (Timeline|Timeline_0 Reverse)
          (else
            (Collision|SetCollisionEnabled _box "QueryAndPhysics")
            (if (Variables|Default|GetEtap)
              ;[0.15 0.15 0.15 0.5] Checking state of buttons
              (for (_array_element _array_index) (Variables|Default|GetButtons)
                (bind _asbp_slider (Utilities|Casting|CastToBP_Slider _array_element))
                (Utilities|Array|SetArrayElem _etap1buttonsstate _array_index (Variables|/Game/Blueprints/BP_Slider.BP_Slider_C|GetIsPressed _asbp_slider)))
              (if (Utilities|Array|Identical (Variables|Default|GetEtap1CorrectPattern) _etap1buttonsstate)
                ;[0.15 0.15 0.15 0.5] light management
                (Rendering|Material|SetMaterial (Variables|Default|GetButton) 0 "/Game/VRTemplate/Materials/M_Green.M_Green")
                (Utilities|FlowControl|Delay 0.1)
                (bind _asdirectional_light (Utilities|Casting|CastToDirectionalLight (Variables|Default|Getlight)))
                (Rendering|Components|Light|SetIntensity (Variables|/Script/Engine.Light|GetLightComponent _asdirectional_light) 0.0)
                (Utilities|FlowControl|Delay 2.0)
                ;[0.15 0.15 0.15 0.5] change of environment
                (bind _asstatic_mesh_actor (Utilities|Casting|CastToStaticMeshActor (Variables|Default|GetChalkBoard)))
                (Rendering|Material|SetMaterial (Variables|/Script/Engine.StaticMeshActor|GetStaticMeshComponent _asstatic_mesh_actor) 0 "/Game/AssetsWeii/RoomBuild/Furniture/Boards/Chalkboard/M_ChalkboardRiddle2.M_ChalkboardRiddle2")
                (bind _asstatic_mesh_actor_2 (Utilities|Casting|CastToStaticMeshActor (Variables|Default|GetWhiteBoard)))
                (Rendering|Material|SetMaterial (Variables|/Script/Engine.StaticMeshActor|GetStaticMeshComponent _asstatic_mesh_actor_2) 0 "/Game/AssetsWeii/RoomBuild/Furniture/Boards/Whiteboard/M_WhiteboardRiddleElectronicLab.M_WhiteboardRiddleElectronicLab")
                (for _array_element_2 (Variables|Default|GetSlidersRef)
                  (if (Variables|/Game/Blueprints/BP_Slider.BP_Slider_C|GetIsPressed _array_element_2)
                    (Variables|/Game/Blueprints/BP_Slider.BP_Slider_C|SetIsPressed _array_element_2 false)
                    (Default|ReversefromEnd _array_element_2)
                    (Collision|SetCollisionEnabled (Variables|Default|GetBox) "NoCollision")
                    ;[0.15 0.15 0.15 0.5] light management
                    (bind _asdirectional_light_2 (Utilities|Casting|CastToDirectionalLight (Variables|Default|Getlight)))
                    (Rendering|Components|Light|SetIntensity (Variables|/Script/Engine.Light|GetLightComponent _asdirectional_light_2) 14.0)
                    (Variables|Default|SetEtap false)))))))))))

(fn ConstructionScript)

(fn RegisterClicked
  (params (ButtonID :type Integer))
  (Utilities|Array|Add (Variables|Default|GetEtap2ButtonOrder) ButtonID))