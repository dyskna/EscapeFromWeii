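; Physical button actor that switches a projector screen between two slides, pressed by overlapping its box.
; An overlap disables the box collision and plays a timeline that pushes the button in.
; At full press it toggles the material on the referenced screen and reverses the timeline, restoring collision once released.
; A MoveButton event slides the whole actor by a given offset to follow an opening drawer.
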(event OnComponentBeginOverlap(Box)
  (params (OverlappedComponent :type Primitive%20Component%20Object%20Reference) (OtherActor :type Actor%20Object%20Reference) (OtherComp :type Primitive%20Component%20Object%20Reference) (OtherBodyIndex :type Integer) (bFromSweep :type Boolean) (SweepResult :type Hit%20Result%20Structure%20%28by%20ref%29))
  (bind _box (Variables|Default|GetBox))
  ;[0.15 0.15 0.15 0.5] Button press animation
  (if (not (Variables|Default|GetIsPressed))
    (Variables|Default|SetIsPressed true)
    (Collision|SetCollisionEnabled _box "NoCollision")
    (bind _alpha (Timeline|Timeline%20Button%20Animation Play)
      (:Update
        (Transformation|SetRelativeLocation (Variables|Default|GetButton) (Math|Vector|Lerp(Vector) "0, 0, 0" "0.000000,-3.000000,0.000000" _alpha) false false))
      (:Finished
        (if (Variables|Default|GetIsPressed)
          (Variables|Default|SetIsPressed false)
          (CallFunction|OnButtonPressed)
          (Timeline|Timeline%20Button%20Animation Reverse)
          (else
            (Collision|SetCollisionEnabled _box "QueryAndPhysics")))))))

(event Custom|OnButtonPressed
  (bind _projectorscreenref (Variables|Default|GetProjectorScreenRef))
  (bind _projectorscreen (Variables|/Game/Blueprints/Screen/ProjectorScreen.ProjectorScreen_C|GetProjectorScreen _projectorscreenref))
  ;[0.15 0.15 0.15 0.5] Changing slides
  (if (Variables|Default|GetFirstSlide)
    (Variables|Default|SetFirstSlide false)
    (Rendering|Material|SetMaterial _projectorscreen 0 "/Game/AssetsWeii/RoomBuild/Furniture/projectorscreen/M_ProjectorScreen1.M_ProjectorScreen1") ; Replace material with second slide
    (else
      (Variables|Default|SetFirstSlide true)
      (Rendering|Material|SetMaterial _projectorscreen 0 "/Game/AssetsWeii/RoomBuild/Furniture/projectorscreen/M_ProjectorScreen.M_ProjectorScreen") ; Replace material with first slide
    )))

(event Custom|MoveButton
  (params (OpenOffset :type Vector))
  ;[0.15 0.15 0.15 0.5] Move the button with the drawer when it opens
  (Variables|Default|SetOriginalButtonLocation (Transformation|GetWorldLocation (Variables|Default|GetDefaultSceneRoot)))
  (bind _alpha (Timeline|Timeline Play)
    (:Update
      (Transformation|SetRelativeLocation (Variables|Default|GetDefaultSceneRoot) (Math|Vector|Lerp(Vector) (Variables|Default|GetOriginalButtonLocation) (+ (Variables|Default|GetOriginalButtonLocation) OpenOffset) _alpha) false false))))

(fn ConstructionScript)