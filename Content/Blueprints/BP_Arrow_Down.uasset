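; Down-arrow actor for a numeric digit display, apparently meant to step the shown number downward.
; Overlapping its Box only destroys Num0 and spawns a Num_1_0 actor.
; An unconnected branch chain, which never runs, swaps the Slot actor for a digit actor 36 units above the Arrow according to Value, then decrements Value, wrapping from 0 to 9.
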(event OnComponentBeginOverlap(Box)
  (params (OverlappedComponent :type Primitive%20Component%20Object%20Reference) (OtherActor :type Actor%20Object%20Reference) (OtherComp :type Primitive%20Component%20Object%20Reference) (OtherBodyIndex :type Integer) (bFromSweep :type Boolean) (SweepResult :type Hit%20Result%20Structure%20%28by%20ref%29))
  (Actor|DestroyActor (Variables|Default|GetNum_0))
  (Game|SpawnActorfromClass "/Game/Blueprints/Numbers/Num_1_0.Num_1_0_C" (Math|Transform|MakeTransform "0, 0, 0" "0, 0, 0" "1.000000,1.000000,1.000000") "Undefined" "MultiplyWithRoot" 0 0))

(fn ConstructionScript)