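; Player pawn for keyboard-and-mouse PC play, handling first-person look, walking and crouching.
; Enhanced Input actions drive yaw/pitch and movement along the actor's forward and right vectors.
; The PC mapping context is added on controller change, and on BeginPlay when no head-mounted display is enabled.
; Crouch uses a custom timeline that lerps capsule half-height and camera height, reversing on release.
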(event Custom|StartCrouch
  ;[0.15 0.15 0.15 0.5] Crouching
  (bind _alpha (Timeline|Timeline%20Crouch Play)
    (:Update
      (Components|Capsule|SetCapsuleHalfHeight (Variables|Collision|GetCapsuleComponent) (Math|Float|Lerp 88.0 44.0 _alpha) true)
      (Transformation|SetRelativeLocation (Variables|Default|GetPlayerCamera) (Math|Vector|Lerp(Vector) "0.000000,0.000000,80.000000" "0.000000,0.000000,40.000000" _alpha) false false))))

(event Custom|EndCrouch
  ;[0.15 0.15 0.15 0.5] Crouching
  (bind _alpha (Timeline|Timeline%20Crouch Reverse)
    (:Update
      (Components|Capsule|SetCapsuleHalfHeight (Variables|Collision|GetCapsuleComponent) (Math|Float|Lerp 88.0 44.0 _alpha) true)
      (Transformation|SetRelativeLocation (Variables|Default|GetPlayerCamera) (Math|Vector|Lerp(Vector) "0.000000,0.000000,80.000000" "0.000000,0.000000,40.000000" _alpha) false false))))

(event Input|EnhancedActionEvents|EnhancedInputActionIA_PCLook
  (params (ActionValue :type Vector%202D%20Structure) (ElapsedSeconds :type Float%20%28double-precision%29) (TriggeredSeconds :type Float%20%28double-precision%29) (InputAction :type Input%20Action%20Object%20Reference :default "/Game/PCControls/Input/Actions/IA_PCLook.IA_PCLook"))
  ;[0.15 0.15 0.15 0.5] Camera movement (looking around)
  (Pawn|Input|AddControllerYawInput (.x ActionValue))
  (Pawn|Input|AddControllerPitchInput (* (.y ActionValue) -1.0)))

(event Input|EnhancedActionEvents|EnhancedInputActionIA_PCMove
  (params (ActionValue :type Vector%202D%20Structure) (ElapsedSeconds :type Float%20%28double-precision%29) (TriggeredSeconds :type Float%20%28double-precision%29) (InputAction :type Input%20Action%20Object%20Reference :default "/Game/PCControls/Input/Actions/IA_PCMove.IA_PCMove"))
  ;[0.15 0.15 0.15 0.5] Movement (walking)
  (Pawn|Input|AddMovementInput (Transformation|GetActorRightVector) (.x ActionValue) false)
  (Pawn|Input|AddMovementInput (Transformation|GetActorForwardVector) (.y ActionValue) false))

(event EventBeginPlay
  ;[0.15 0.15 0.15 0.5] Keyboard mapping on startup (when VR headset not detected)
  (if (not (Class|HeadMountedDisplayFunctionLibrary|IsHeadMountedDisplayEnabled))
    (Input|AddMappingContext (PlayerController|LocalPlayerSubsystems|GetEnhancedInputLocalPlayerSubsystem (Game|GetPlayerController 0)) "/Game/PCControls/Input/IMC_PCDefault.IMC_PCDefault" 0 "(bIgnoreAllPressedKeysUntilRelease=True,bForceImmediately=False,bNotifyUserSettings=False)")))

(event EventControllerChanged
  (params (OldController :type Controller%20Object%20Reference) (NewController :type Controller%20Object%20Reference))
  ;[0.15 0.15 0.15 0.5] Keyboard mapping on controller change
  (bind _asplayer_controller (Utilities|Casting|CastToPlayerController NewController))
  (Input|AddMappingContext (PlayerController|LocalPlayerSubsystems|GetEnhancedInputLocalPlayerSubsystem _asplayer_controller) "/Game/PCControls/Input/IMC_PCDefault.IMC_PCDefault" 0 "(bIgnoreAllPressedKeysUntilRelease=True,bForceImmediately=False,bNotifyUserSettings=False)"))

(event Input|ActionEvents|InputActionCrouch
  (params (Key :type Key%20Structure :default "None"))
  ;[0.15 0.15 0.15 0.5] Crouching
  (:Pressed
    (CallFunction|StartCrouch))
  (:Released
    (CallFunction|EndCrouch)))

(fn ConstructionScript)